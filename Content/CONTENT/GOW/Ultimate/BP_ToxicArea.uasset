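; BP_ToxicArea is a timed toxic area attack that rains BP_ToxicSpear actors from above.
; BeginPlay creates dynamic materials for the cloud and ground, with the ground faint until BeginAttack brightens it.
; BeginAttack starts a rapid looping timer that spawns downward-pitched spears at random offsets above the cloud, plus a timer for Death.
; Death stops spawning, waits briefly, fades both materials out with a timeline, then destroys the actor.
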(event `self.ReceiveBeginPlay`
  (bind _returnvalue (`KismetMaterialLibrary.CreateDynamicMaterialInstance` "/Game/CONTENT/GOW/Ultimate/MI_ToxicCloud.MI_ToxicCloud"))
  (bind _output_get (set `self.CloudMat` _returnvalue))
  (`PrimitiveComponent.SetMaterial` (`self.Cloud`) 0 _output_get)
  (bind _returnvalue_2 (`KismetMaterialLibrary.CreateDynamicMaterialInstance` "/Game/CONTENT/GOW/Ultimate/M_ToxinArea.M_ToxinArea"))
  (bind _output_get_2 (set `self.GroundMat` _returnvalue_2))
  (`PrimitiveComponent.SetMaterial` (`self.Ground`) 0 _output_get_2)
  (`MaterialInstanceDynamic.SetScalarParameterValue` (`self.GroundMat`) "Opacity" 0.1))

(event `Death`
  (`KismetSystemLibrary.K2_ClearAndInvalidateTimerHandle` (`self.Atack Spawn`))
  (`KismetSystemLibrary.Delay` 1.65)
  (bind (_direction _newtrack_0) (`Timeline|Timeline` :!via `PlayFromStart`)
    (:`Update`
      (`MaterialInstanceDynamic.SetScalarParameterValue` (`self.CloudMat`) "Opacity" (`KismetMathLibrary.Lerp` 0.9 0.0 _newtrack_0))
      (`MaterialInstanceDynamic.SetScalarParameterValue` (`self.GroundMat`) "Opacity" (`KismetMathLibrary.Lerp` 0.2 0.0 _newtrack_0)))
    (:`Finished`
      (`self.K2_DestroyActor`))))

(event `Begin Attack`
  (`MaterialInstanceDynamic.SetScalarParameterValue` (`self.GroundMat`) "Opacity" 0.25)
  (`KismetSystemLibrary.K2_SetTimerDelegate` (delegate `Death`) 8.0)
  (bind _returnvalue (`KismetSystemLibrary.K2_SetTimerDelegate` (delegate `Killing`) 0.075 true))
  (set `self.Atack Spawn` _returnvalue))

(event `Killing`
  (`|SpawnActorFromClass` "/Game/CONTENT/GOW/Ultimate/BP_ToxicSpear.BP_ToxicSpear_C" (`KismetMathLibrary.MakeTransform` (+ (`SceneComponent.K2_GetComponentLocation` (`self.Cloud`)) (`KismetMathLibrary.MakeVector` (`KismetMathLibrary.RandomFloatInRange` -450.0 450.0) (`KismetMathLibrary.RandomFloatInRange` -450.0 450.0) 1500.0)) (`KismetMathLibrary.MakeRotator` (`KismetMathLibrary.RandomFloatInRange` -45.0 45.0) -90.0 (`KismetMathLibrary.RandomFloatInRange` -45.0 45.0))) "Undefined" "MultiplyWithRoot" null null))

(fn `UserConstructionScript`)