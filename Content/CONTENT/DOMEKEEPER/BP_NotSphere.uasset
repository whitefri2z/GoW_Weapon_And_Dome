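; BP_NotSphere is an actor in the DOMEKEEPER folder that aims an arrow at the mouse cursor.
; BeginPlay spawns a CameraActor at its camera component, makes it the view target and shows the cursor.
; Tick pitches the arrow by the cursor's atan2 angle, assuming a 1920x1080 viewport, and prints it for debugging.
; The Centred flag selects screen centre or bottom-centre as pivot, and the construction script shifts the sphere to match.
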(event `self.ReceiveBeginPlay`
  (bind _returnvalue (`GameplayStatics.GetPlayerController` 0))
  (bind _returnvalue_2 (`|SpawnActorFromClass` "/Script/Engine.CameraActor" (`SceneComponent.K2_GetComponentToWorld` (`self.Camera`)) "Undefined" "MultiplyWithRoot" null null))
  (`PlayerController.SetViewTargetWithBlend` _returnvalue _returnvalue_2 0.0 "VTBlend_Linear" 0.0 false)
  (set `PlayerController.bShowMouseCursor` true _returnvalue))

(event `self.ReceiveTick`
  (params (DeltaSeconds :type "Float (single-precision)"))
  (bind _returnvalue (`WidgetLayoutLibrary.GetMousePositionOnViewport`))
  (bind (_x _y) (`KismetMathLibrary.BreakVector2D` _returnvalue))
  (bind _returnvalue_2 (- (`KismetMathLibrary.DegAtan2` (- _x (/ 1920.0 2.0)) (- _y (`KismetMathLibrary.SelectFloat` 540.0 1080.0 (`self.Centred`)))) 90.0))
  (`SceneComponent.K2_SetRelativeRotation` (`self.Arrow`) (`KismetMathLibrary.MakeRotator` 0.0 _returnvalue_2) false false)
  (`KismetSystemLibrary.PrintString` (`KismetStringLibrary.Conv_DoubleToString` _returnvalue_2) true true (struct :`R` 1.0 :`G` 0.982079 :`A` 1.0) 0.0))

(fn `UserConstructionScript`
  (`SceneComponent.K2_SetRelativeLocation` (`self.Sphere`) (`KismetMathLibrary.MakeVector` 0.0 0.0 (`KismetMathLibrary.SelectFloat` 0.0 -430.0 (`self.Centred`))) false false))